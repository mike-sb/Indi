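; Inventory actor component that lets its owning first-person character look at and interact with items and keep a list of item slots.
; Each tick a camera-forward sphere trace (debug drawn) updates the looked-at actor and shows its message in a UW_Message widget.
; The Interact input passes the character to that actor's AC_Item_Data component.
; AddToInventory appends slots by item name, and QueryInventory checks for a name.
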(event `self.ReceiveBeginPlay`
  (`KismetArrayLibrary.Array_Resize` (`self.Content`))
  (bind _returnvalue (`|CreateWidget` "/Game/Inventory/UI/UW_Message.UW_Message_C"))
  (bind _output_get (set `self.DisplayMessage` _returnvalue))
  (`UserWidget.AddToViewport` _output_get 0))

(event `self.ReceiveTick`
  (params (DeltaSeconds :type "Float (single-precision)"))
  (`self.InteractionTrace`))

(event `InputAction|Interact`
  (params (Key :type "Key Structure"))
  (:`Pressed`
    (bind _lookatactor (`self.LookAtActor`)
      (:`then`
        (bind _returnvalue (`Actor.GetComponentByClass` _lookatactor "/Game/Inventory/AC_Item_Data.AC_Item_Data_C"))
        (`/Engine/EditorBlueprintResources/StandardMacros.IsValid` _returnvalue
          (:`Is Valid`
            (bind _asbp_first_person_character (cast `/Game/FirstPerson/Blueprints/BP_FirstPersonCharacter` (`self.GetOwner`)))
            (message `/Game/Inventory/I_Interact.InteractWith` _returnvalue _asbp_first_person_character))))
      (:`else`))))

(fn `AddToInventory`
  (params (ItemName :type Name))
  (`KismetArrayLibrary.Array_Add` (`self.Content`) (make `/Game/Inventory/FSlotStruct` ItemName)))

(fn `InteractionTrace`
  (bind _returnvalue (`GameplayStatics.GetPlayerCameraManager` 0))
  (bind _returnvalue_2 (`Actor.K2_GetActorLocation` _returnvalue))
  (bind (_outhit _returnvalue_3) (`KismetSystemLibrary.SphereTraceSingle` _returnvalue_2 (+ _returnvalue_2 (* (`Actor.GetActorForwardVector` _returnvalue) 300.0)) 10.0 "TraceTypeQuery3" false (`|MakeArray` (`self.GetOwner`)) "ForOneFrame"))
  (if _returnvalue_3
    (bind (_bblockinghit _binitialoverlap _time _distance _location _impactpoint _normal _impactnormal _physmat _hitactor) (`GameplayStatics.BreakHitResult` _outhit))
    (if (!= _hitactor (`self.LookAtActor`))
      (bind _output_get (set `self.LookAtActor` _hitactor))
      (bind _message (message `/Game/Inventory/I_Interact.LookAt` _output_get))
      (`/Game/Inventory/UI/UW_Message.ShowMessage` (`self.DisplayMessage`) _message))
    (else
      (set `self.LookAtActor` null)
      (`/Game/Inventory/UI/UW_Message.ShowMessage` (`self.DisplayMessage`) ""))))

(fn `QueryInventory`
  (params (ItemName :type Name))
  (returns (Success :type Boolean))
  (for _array_element (`self.Content`)
    (if (== (`.ItemName_2_2FB955374C48E52C444F6986B679A6E8` (break `/Game/Inventory/FSlotStruct` _array_element)) ItemName)
      (return true)))
  (return false))