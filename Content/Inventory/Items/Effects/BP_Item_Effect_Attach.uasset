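; BP_Item_Effect_Attach is an inventory item effect that attaches the used item to the player character.
; Its UseItem event casts player 0 to BP_FirstPersonCharacter and sets the class of the child actor component from GetItemSlot to the given item.
; It then disables collision on the spawned child actor and removes the item at the given index from the character's inventory system.
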(event `self.UseItem`
  (params (Item :type "Actor Class Reference") (Index :type Integer))
  (set `self.Index` Index)
  (bind _asbp_first_person_character (cast `/Game/FirstPerson/Blueprints/BP_FirstPersonCharacter` (`GameplayStatics.GetPlayerCharacter` 0)))
  (bind _itemslot (`/Game/FirstPerson/Blueprints/BP_FirstPersonCharacter.GetItemSlot` _asbp_first_person_character))
  (`ChildActorComponent.SetChildActorClass` _itemslot Item)
  (`self.SetActorEnableCollision` (`ChildActorComponent.ChildActor` _itemslot) false)
  (`/Game/Inventory/AC_Inventory_System.RemoveItem` (`/Game/FirstPerson/Blueprints/BP_FirstPersonCharacter.AC_Inventory_System` _asbp_first_person_character) (`self.Index`)))

(fn `UserConstructionScript`
  (`parent.UserConstructionScript`))