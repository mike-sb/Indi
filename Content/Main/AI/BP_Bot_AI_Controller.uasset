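; BP_Bot_AI_Controller is the AI controller for bots, running the BT_Bot behavior tree on BeginPlay.
; Its AI Perception component writes any successfully sensed actor to the Player blackboard key and clears that key when a stimulus is lost.
; The sensed actor is stored without filtering by type or sense, and debug prints report the sense class and each value set.
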(event `self.ReceiveBeginPlay`
  (`self.RunBehaviorTree` "/Game/Main/AI/BT_Bot.BT_Bot"))

(event `self.AIPerception.OnTargetPerceptionUpdated`
  (params (Actor :type "Actor Object Reference") (Stimulus :type "AIStimulus Structure"))
  (bind _returnvalue (`AIBlueprintHelperLibrary.GetBlackboard` null))
  (bind _returnvalue_2 (`KismetStringLibrary.Conv_StringToName` "Player"))
  (bind _returnvalue_3 (`AIPerceptionSystem.GetSenseClassForStimulus` Stimulus))
  (`KismetSystemLibrary.PrintString` (`KismetSystemLibrary.GetClassDisplayName` _returnvalue_3))
  (if (`.bSuccessfullySensed` (break `AIStimulus` Stimulus))
    (`BlackboardComponent.SetValueAsObject` _returnvalue _returnvalue_2 Actor)
    (`KismetSystemLibrary.PrintString` "Value Set")
    (else
      (`BlackboardComponent.ClearValue` _returnvalue _returnvalue_2))))

(fn `UserConstructionScript`)