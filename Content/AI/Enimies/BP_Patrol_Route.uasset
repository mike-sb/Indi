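; BP_Patrol_Route is a placeable patrol route for enemy AI, defined by a spline whose points serve as waypoints.
; GetSplinePointAsPosition returns the world location of the spline point at the current Index.
; IncrementRoute steps Index by Direction and flips Direction at the last and first points, so the route is traversed back and forth rather than looped.
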(event `IncrementRoute`
  (bind _output_get (set `self.index` (+ (`self.index`) (`self.direction`))))
  (if (== _output_get (- (`SplineComponent.GetNumberOfSplinePoints` (`self.PatroleRoute`)) 1))
    (set `self.direction` -1)
    (elif (== (`self.index`) 0)
      (set `self.direction` 1))))

(fn `GetSplinePointAsPosition`
  (returns (Loacation :type "Vector Structure"))
  (return (`SplineComponent.GetLocationAtSplinePoint` (`self.PatroleRoute`) (`self.index`) "World")))

(fn `UserConstructionScript`)