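; AI controller for a camera bot that switches to attack when it spots the player.
; On BeginPlay it runs BT_Camera and sets the blackboard State to Passive.
; Perception updates are filtered to successful sight stimuli; if the first player character is seen while Passive, it writes the Attack state, target and stimulus location to the blackboard.
; Nothing here returns it to Passive after that switch.
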(event `self.ReceiveBeginPlay`
  (`self.RunBehaviorTree` "/Game/AI/Camera/BT_Camera.BT_Camera")
  (`self.SetStateAsPassive`))

(event `self.AIPerception.OnPerceptionUpdated`
  (params (UpdatedActors :type "Array of Actor Object Reference (by ref)"))
  (for _array_element UpdatedActors
    (bind (_issensed _stimulus) (`self.CanSenseActor` _array_element))
    (if _issensed
      (`self.HandleSenseSight` _array_element (`.StimulusLocation` (break `AIStimulus` _stimulus))))))

(fn `CanSenseActor`
  (params (Actor :type "Actor Object Reference") (Sense :type "/Game/AI/Enimies/Enums/E_AI_Sense Enum" :default "NewEnumerator0"))
  (returns (isSensed :type Boolean) (Stimulus :type "AIStimulus Structure"))
  (bind _info (`AIPerceptionComponent.GetActorsPerception` (`self.AIPerception`) Actor))
  (for _array_element (`.LastSensedStimuli` (break `ActorPerceptionBlueprintInfo` _info))
    (bind _returnvalue (`AIPerceptionSystem.GetSenseClassForStimulus` _array_element))
    (if (== _returnvalue (select `/Game/AI/Enimies/Enums/E_AI_Sense` Sense :`NewEnumerator0` "/Script/AIModule.AISense_Sight" :`NewEnumerator1` "/Script/AIModule.AISense_Hearing" :`NewEnumerator2` "/Script/AIModule.AISense_Damage" :!type "AISense Class Reference"))
      (return (`.bSuccessfullySensed` (break `AIStimulus` _array_element)) _array_element))))

(fn `GetCurrentState`
  (returns (State :type "/Game/AI/Enimies/Enums/E_BotStates Enum"))
  (return (cast `/Game/AI/Enimies/Enums/E_BotStates` (`BlackboardComponent.GetValueAsEnum` (`AIBlueprintHelperLibrary.GetBlackboard` null) (`KismetStringLibrary.Conv_StringToName` "State")))))

(fn `HandleSenseSight`
  (params (Actor :type "Actor Object Reference") (Point :type "Vector Structure"))
  (if (== Actor (`GameplayStatics.GetPlayerCharacter` 0))
    (bind _state (`self.GetCurrentState`))
    (switch `/Game/AI/Enimies/Enums/E_BotStates` _state
      (:`NewEnumerator0`
        (`self.SetStateAsAttacking` Actor Point)))))

(fn `SetStateAsAttacking`
  (params (AttackTarget :type "Actor Object Reference") (Point :type "Vector Structure"))
  (locals (Player :type Name :default "Player") (State :type Name :default "State") (PointOfInterest :type Name :default "PointOfInterest"))
  (bind _returnvalue (`AIBlueprintHelperLibrary.GetBlackboard` null))
  (`BlackboardComponent.SetValueAsEnum` _returnvalue (`local.State`) (enumliteral `/Game/AI/Enimies/Enums/E_BotStates` "NewEnumerator1"))
  (`BlackboardComponent.SetValueAsObject` _returnvalue (`local.Player`) AttackTarget)
  (`BlackboardComponent.SetValueAsVector` _returnvalue (`local.PointOfInterest`) Point))

(fn `SetStateAsPassive`
  (`BlackboardComponent.SetValueAsEnum` (`AIBlueprintHelperLibrary.GetBlackboard` null) (`KismetStringLibrary.Conv_StringToName` "State") (enumliteral `/Game/AI/Enimies/Enums/E_BotStates` "NewEnumerator0")))

(fn `UserConstructionScript`)